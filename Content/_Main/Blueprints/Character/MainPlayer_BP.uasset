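; Main player character Blueprint that sets up hero stats from a player class and includes a debug damage key.
; On BeginPlay, a switch on the class enum builds the hero struct, with only the Sourcerer case filled in, then passes it to InitializeCharacter.
; Pressing 1 applies test damage to itself, subtracts the returned amount from current health and prints the result.
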(event `self.ReceiveBeginPlay`
  (`|ExecutionSequence`
    (:`then_0`
      (switch `/Game/_Main/Blueprints/Program/HeroClass_E` (`self.E_PlayerClass`)
        (:`NewEnumerator0`
          (bind _output_get (set `self.FStructHero` (make `StructHero` 0.0 0.0 0.0 100.0 0.0 100.0 0.0 100.0 0.0 0.8))))))
    (:`then_1`
      (`self.InitializeCharacter` (`self.FStructHero`)))))

(event `Key|One`
  (params (Key :type "Key Structure"))
  (:`Pressed`
    (bind _returnvalue (`GameplayStatics.ApplyDamage` self 10.0))
    (bind _output_get (set `self.fCHealth` (- (`self.fCHealth`) _returnvalue)))
    (`KismetSystemLibrary.PrintString` (`KismetStringLibrary.Conv_DoubleToString` _output_get))))

(fn `UserConstructionScript`)